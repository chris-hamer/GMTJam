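; Player dodge state that briefly launches the character at high speed, then returns it to the Normal state.
; Enter calls SwitchCharacter, locks in the movement input (or backward from facing when idle), spawns a woosh, boosts speed and acceleration, and ignores Pawn collision.
; TickState feeds that fixed direction into movement until a short timer ends the dodge.
; Exit sets walk speed and acceleration to hardcoded values and blocks Pawns again.
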(event Custom|EndDodge
  (Default|SetState (Variables|Default|GetPlayer) "Normal"))

(event EventExit
  (params (PlayerCharacter :type Top%20Down%20Character%20Object%20Reference))
  (bind _player (Variables|Default|GetPlayer))
  (bind _charactermovement (Variables|/Script/Engine.Character|GetCharacterMovement _player))
  (Variables|/Script/Engine.CharacterMovementComponent|SetMaxWalkSpeed _charactermovement 6e+02)
  (Variables|/Script/Engine.CharacterMovementComponent|SetMaxAcceleration _charactermovement 2048.0)
  (Collision|SetCollisionResponsetoChannel (Variables|/Script/Engine.Character|GetCapsuleComponent _player) "ECC_Pawn" "ECR_Block"))

(event EventTickState
  (params (PlayerCharacter :type Top%20Down%20Character%20Object%20Reference))
  (Class|PawnMovementComponent|AddInputVector (Variables|/Script/Engine.Character|GetCharacterMovement (Variables|Default|GetPlayer)) (* (Variables|Default|GetInitial%20Input) 2.0) false))

(event EventEnter
  (params (PlayerCharacter :type Top%20Down%20Character%20Object%20Reference))
  (bind _movementinput (Variables|/Game/Blueprints/TopDownCharacter.TopDownCharacter_C|GetMovementInput PlayerCharacter))
  (Variables|Default|SetPlayer PlayerCharacter)
  (Default|SwitchCharacter (Variables|Default|GetPlayer))
  (Variables|Default|SetInitial%20Input (Math|Vector|ClampVectorSize (select (Math|Vector|Equal(Vector) "0, 0, 0" _movementinput 0.0001) (* (Math|Vector|GetForwardVector (Variables|/Script/Engine.Character|GetCapsuleComponent PlayerCharacter)) -1.0) _movementinput) 0.0 1.0))
  (Utilities|Time|SetTimerbyEvent (delegate Custom|EndDodge) 0.25)
  (Variables|/Script/Engine.CharacterMovementComponent|SetMaxWalkSpeed (Variables|/Script/Engine.Character|GetCharacterMovement (Variables|Default|GetPlayer)) 1.8e+03)
  (Variables|/Script/Engine.CharacterMovementComponent|SetMaxAcceleration (Variables|/Script/Engine.Character|GetCharacterMovement (Variables|Default|GetPlayer)) 1e+04)
  (Default|SpawnWoosh (Variables|Default|GetPlayer) (Variables|Default|GetInitial%20Input))
  (Collision|SetCollisionResponsetoChannel (Variables|/Script/Engine.Character|GetCapsuleComponent (Variables|Default|GetPlayer)) "ECC_Pawn" "ECR_Ignore"))
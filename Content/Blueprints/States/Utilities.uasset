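; Utility Blueprint for player states with one function, ConsumeStamina, which spends stamina for the player's active character.
; It switches on CurrentCharacter to pick one of two separate pools, Stamina1 or Stamina2.
; The cost is subtracted only when the pool is strictly greater than it; otherwise nothing changes and no result is returned to the caller.
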(fn ConsumeStamina
  (params (Player :type Top%20Down%20Character%20Object%20Reference) (StaminaCost :type Float%20%28single-precision%29))
  (switch Utilities|FlowControl|Switch|SwitchonCharacters (Variables|/Game/Blueprints/TopDownCharacter.TopDownCharacter_C|GetCurrentCharacter Player)
    (:NewEnumerator0
      (if (> (Variables|/Game/Blueprints/TopDownCharacter.TopDownCharacter_C|GetStamina1 Player) StaminaCost)
        (Variables|/Game/Blueprints/TopDownCharacter.TopDownCharacter_C|SetStamina1 Player (- (Variables|/Game/Blueprints/TopDownCharacter.TopDownCharacter_C|GetStamina1 Player) StaminaCost))))
    (:NewEnumerator1
      (if (> (Variables|/Game/Blueprints/TopDownCharacter.TopDownCharacter_C|GetStamina2 Player) StaminaCost)
        (Variables|/Game/Blueprints/TopDownCharacter.TopDownCharacter_C|SetStamina2 Player (- (Variables|/Game/Blueprints/TopDownCharacter.TopDownCharacter_C|GetStamina2 Player) StaminaCost))))))